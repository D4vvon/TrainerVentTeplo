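; BP_Shtorki is an interactable mechanism of louvre-style shutters ("shtorki"), built from the main ComponentMesh and four slat elements, El1 to El4.
; OpenShtroki and CloseShtorki step CurrentAngle one degree per call within MinAngle and MaxAngle, rolling all five parts together.
; Tick copies ComponentMesh's first material onto the four elements every frame, keeping their look in sync.
; Nothing in this Blueprint calls the open or close functions.
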(event `self.ReceiveTick`
  (params (DeltaSeconds :type "Float (single-precision)"))
  (bind _returnvalue (`PrimitiveComponent.GetMaterial` (`self.ComponentMesh`) 0))
  (`PrimitiveComponent.SetMaterial` (`self.El1`) 0 _returnvalue)
  (`PrimitiveComponent.SetMaterial` (`self.El2`) 0 _returnvalue)
  (`PrimitiveComponent.SetMaterial` (`self.El3`) 0 _returnvalue)
  (`PrimitiveComponent.SetMaterial` (`self.El4`) 0 _returnvalue))

(fn `Close Shtorki`
  (bind _currentangle (`self.CurrentAngle`))
  (if (> (`self.CurrentAngle`) (`self.MinAngle`))
    (set `self.CurrentAngle` (- (`self.CurrentAngle`) 1.0))
    (`SceneComponent.K2_SetRelativeRotation` (`self.El1`) (`KismetMathLibrary.MakeRotator` _currentangle) false false)
    (`SceneComponent.K2_SetRelativeRotation` (`self.El2`) (`KismetMathLibrary.MakeRotator` _currentangle) false false)
    (`SceneComponent.K2_SetRelativeRotation` (`self.El3`) (`KismetMathLibrary.MakeRotator` _currentangle) false false)
    (`SceneComponent.K2_SetRelativeRotation` (`self.El4`) (`KismetMathLibrary.MakeRotator` _currentangle) false false)
    (`SceneComponent.K2_SetRelativeRotation` (`self.ComponentMesh`) (`KismetMathLibrary.MakeRotator` _currentangle) false false)))

(fn `OpenShtroki`
  (bind _currentangle (`self.CurrentAngle`))
  (if (< (`self.CurrentAngle`) (`self.MaxAngle`))
    (set `self.CurrentAngle` (+ (`self.CurrentAngle`) 1.0))
    (`SceneComponent.K2_SetRelativeRotation` (`self.El1`) (`KismetMathLibrary.MakeRotator` _currentangle) false false)
    (`SceneComponent.K2_SetRelativeRotation` (`self.El2`) (`KismetMathLibrary.MakeRotator` _currentangle) false false)
    (`SceneComponent.K2_SetRelativeRotation` (`self.El3`) (`KismetMathLibrary.MakeRotator` _currentangle) false false)
    (`SceneComponent.K2_SetRelativeRotation` (`self.El4`) (`KismetMathLibrary.MakeRotator` _currentangle) false false)
    (`SceneComponent.K2_SetRelativeRotation` (`self.ComponentMesh`) (`KismetMathLibrary.MakeRotator` _currentangle) false false)))

(fn `UserConstructionScript`)