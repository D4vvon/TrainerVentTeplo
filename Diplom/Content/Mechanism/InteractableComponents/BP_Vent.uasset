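; BP_Vent is a ventilation fan among the interactable mechanism components, built from separate meshes for wire, motor, mount, grille, blade hub and five blades.
; Every Tick, it copies the first material of ComponentMesh onto each of these parts, so the whole fan mirrors that mesh's current material.
; The graph holds no rotation or interaction logic, and the construction script is empty.
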(event `self.ReceiveTick`
  (params (DeltaSeconds :type "Float (single-precision)"))
  (bind _returnvalue (`PrimitiveComponent.GetMaterial` (`self.ComponentMesh`) 0))
  (`PrimitiveComponent.SetMaterial` (`self.Provod`) 0 _returnvalue)
  (`PrimitiveComponent.SetMaterial` (`self.OsnovanieLopostei`) 0 _returnvalue)
  (`PrimitiveComponent.SetMaterial` (`self.Lopost1`) 0 _returnvalue)
  (`PrimitiveComponent.SetMaterial` (`self.Lopost2`) 0 _returnvalue)
  (`PrimitiveComponent.SetMaterial` (`self.Lopost3`) 0 _returnvalue)
  (`PrimitiveComponent.SetMaterial` (`self.Lopost4`) 0 _returnvalue)
  (`PrimitiveComponent.SetMaterial` (`self.Lopost5`) 0 _returnvalue)
  (`PrimitiveComponent.SetMaterial` (`self.Reshetka`) 0 _returnvalue)
  (`PrimitiveComponent.SetMaterial` (`self.Kreplenie`) 0 _returnvalue)
  (`PrimitiveComponent.SetMaterial` (`self.Motor`) 0 _returnvalue))

(fn `UserConstructionScript`)